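; Base HUD Blueprint that owns the character info and death pop-up widgets and keeps them in step with player events.
; On BeginPlay it caches GM_Base and binds to its character spawn dispatcher, then creates both widgets on spawn and calls CreatedWidget.
; Character dispatchers drive the UI: hits hide a life, life gains show one, and death starts the pop-up.
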(event `self.ReceiveBeginPlay`
  (`self.GetReferences`)
  (add `/Game/Blueprints/GameModes/GM_Base.OnCharacterSpawn` (`self.As GM Base`) (`|CreateDelegate` :!event `OnCharacterSpawn`)))

(event `OnCharacterSpawn`
  (bind _characterreference (`/Game/Blueprints/GameModes/GM_Base.CharacterReference` (`self.As GM Base`)))
  (`self.CreateWidgets`)
  (add `/Game/Blueprints/Characters/BP_BaseCharacter.TriggerHit` _characterreference (delegate `CustomEvent_0`))
  (add `/Game/Blueprints/Characters/BP_BaseCharacter.TriggerDeath` _characterreference (delegate `TriggerDeath_Event`))
  (add `/Game/Blueprints/Characters/BP_BaseCharacter.IncreaseLife` _characterreference (delegate `IncreseLife`)))

(event `TriggerDeath_Event`
  (`/Game/Widgets/WBP_DeathRoasted.StartPopUp` (`self.DeatWidget`)))

(event `CustomEvent_0`
  (`/Game/Widgets/WBP_CharaceterInfo.HideLife` (`self.Character Info Widget`)))

(event `IncreseLife`
  (`/Game/Widgets/WBP_CharaceterInfo.ShowLife` (`self.Character Info Widget`)))

(fn `CreateWidgets`
  (bind _returnvalue (`|CreateWidget` "/Game/Widgets/WBP_CharaceterInfo.WBP_CharaceterInfo_C"))
  (bind _output_get (set `self.Character Info Widget` _returnvalue))
  (`UserWidget.AddToViewport` _output_get 0)
  (bind _returnvalue_2 (`|CreateWidget` "/Game/Widgets/WBP_DeathRoasted.WBP_DeathRoasted_C"))
  (bind _output_get_2 (set `self.DeatWidget` _returnvalue_2))
  (`UserWidget.AddToViewport` _output_get_2 0)
  (`self.CreatedWidget`))

(fn `GetReferences`
  (bind _asgm_base (cast `/Game/Blueprints/GameModes/GM_Base` (`GameplayStatics.GetGameMode`)))
  (set `self.As GM Base` _asgm_base))

(fn `UserConstructionScript`)