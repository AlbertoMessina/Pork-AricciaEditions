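; Editor layout tool that scatters copies of a chosen static mesh and material along a spline, snapped to the surface below.
; The construction script derives the instance count from spline length and spacing (mesh X size plus an offset).
; At each step it traces down on Visibility and adds an instanced mesh at the hit, raised by half the scaled Y extent, with fixed rotation.
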(fn `UserConstructionScript`
  (locals (NumberOfInstance :type Integer :default 0))
  (bind _instancedstaticmesh (`self.InstancedStaticMesh`))
  (bind (_returnvalue_min _returnvalue_max) (break `Box` (`StaticMesh.GetBoundingBox` (`self.Static Mesh`))))
  (bind (_returnvalue_min_2 _returnvalue_max_2) (break `Box` (`StaticMesh.GetBoundingBox` (`self.Static Mesh`))))
  (`StaticMeshComponent.SetStaticMesh` _instancedstaticmesh (`self.Static Mesh`))
  (`PrimitiveComponent.SetMaterial` _instancedstaticmesh 0 (`self.Static Mesh Material`))
  (bind _output_get (set `self.Spacing` (+ (.x (- _returnvalue_max_2 _returnvalue_min_2)) (`self.offset`))))
  (bind _output_get_2 (set `local.NumberOfInstance` (`KismetMathLibrary.FFloor` (/ (`SplineComponent.GetSplineLength` (`self.Spline`)) _output_get))))
  (for _index (range (+ _output_get_2 1))
    (bind (_returnvalue_location _returnvalue_rotation _returnvalue_scale) (`KismetMathLibrary.BreakTransform` (`KismetMathLibrary.MakeTransform` (`SplineComponent.GetLocationAtDistanceAlongSpline` (`self.Spline`) (* _index (`self.Spacing`)) "World") (struct :`Yaw` 90.0 :`Roll` 90.0))))
    (bind _outhit (`KismetSystemLibrary.LineTraceSingle` _returnvalue_location (- _returnvalue_location (0.0 0.0 1000.0)) "TraceTypeQuery1"))
    (`InstancedStaticMeshComponent.AddInstance` (`self.InstancedStaticMesh`) (`KismetMathLibrary.MakeTransform` (+ (`.Location` (`GameplayStatics.BreakHitResult` _outhit)) (`KismetMathLibrary.MakeVector` 0.0 0.0 (* (/ (.y (- _returnvalue_max _returnvalue_min)) 2.0) (`self.MeshScaleMultiply`)))) _returnvalue_rotation (* _returnvalue_scale (`self.MeshScaleMultiply`))) true)))