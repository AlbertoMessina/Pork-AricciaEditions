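; BP_KosoSparato is a physics-driven projectile in the Traps folder that bursts on hitting a character.
; SetMesh swaps its mesh and rotation and configures physics and collision, while AddImpulse launches it along actor forward as a velocity change.
; A BeginPlay lifetime timer or a hit on a BP_BaseCharacter triggers AutoDestroy, which spawns a hay explosion effect and destroys the actor.
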(event `self.ReceiveBeginPlay`
  (`PrimitiveComponent.SetSimulatePhysics` (`self.StaticMesh`) true)
  (`KismetSystemLibrary.K2_SetTimerDelegate` (delegate `AutoDestroy`) (`self.Lifetime`)))

(event `AutoDestroy`
  (bind _staticmesh (`self.StaticMesh`))
  (`NiagaraFunctionLibrary.SpawnSystemAtLocation` "/Game/VFX/VFX_HayExplosion.VFX_HayExplosion" (`SceneComponent.K2_GetComponentLocation` _staticmesh) (`SceneComponent.K2_GetComponentRotation` _staticmesh))
  (`self.K2_DestroyActor` self))

(event `self.StaticMesh.OnComponentHit`
  (params (HitComponent :type "PrimitiveComponent Object Reference") (OtherActor :type "Actor Object Reference") (OtherComp :type "PrimitiveComponent Object Reference") (NormalImpulse :type "Vector Structure") (Hit :type "HitResult Structure (by ref)"))
  (cast `/Game/Blueprints/Characters/BP_BaseCharacter` OtherActor)
  (`self.AutoDestroy`))

(fn `AddImpulse`
  (params (ForceImpulse :type "Float (single-precision)"))
  (`PrimitiveComponent.AddImpulse` (`self.StaticMesh`) (* (`self.GetActorForwardVector` self) ForceImpulse) "None" true))

(fn `SetMesh`
  (params (NewMesh :type "StaticMesh Object Reference") (NewRotation :type "Rotator Structure"))
  (bind _staticmesh (`self.StaticMesh`))
  (`StaticMeshComponent.SetStaticMesh` _staticmesh NewMesh)
  (`SceneComponent.K2_SetWorldRotation` _staticmesh NewRotation false false)
  (`PrimitiveComponent.SetSimulatePhysics` _staticmesh true)
  (`PrimitiveComponent.SetCollisionResponseToChannel` _staticmesh "ECC_WorldStatic" "ECR_Block")
  (set `PrimitiveComponent.bGenerateOverlapEvents` true _staticmesh)
  (`PrimitiveComponent.SetCollisionObjectType` (`self.StaticMesh`) "ECC_GameTraceChannel1"))

(fn `UserConstructionScript`)