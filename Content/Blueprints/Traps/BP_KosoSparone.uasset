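; BP_KosoSparone is a trap that, once activated, launches BP_KosoSparato projectiles.
; Activation fires immediately and starts a looping timer with an interval randomized once between min and max.
; Each shot gets a random yaw spread, the configured mesh, random uniform scale and a random impulse along its right vector.
; DestroyNearActor can remove other launchers within DeathArea, but is not called here.
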(event `self.ReceiveBeginPlay`)

(event `StartSpawn`)

(event `/Game/Blueprints/Traps/BPI_Trap.Activate`
  (if (not (`self.bActive`))
    (set `self.bActive` true)
    (`self.SpawnBall`)
    (`KismetSystemLibrary.K2_SetTimerDelegate` (`|CreateDelegate` :!event `SpawnBall`) (`KismetMathLibrary.RandomFloatInRange` (`self.MinSpawnTime`) (`self.MaxSpawnTime`)) true)))

(event `SpawnBall`
  (bind (_returnvalue_roll _returnvalue_pitch _returnvalue_yaw) (`KismetMathLibrary.BreakRotator` (`self.K2_GetActorRotation`)))
  (bind _zspawnrotationoffset (`self.ZSpawnRotationOffset`))
  (bind _returnvalue (`|SpawnActorFromClass` (`self.SpawnedClass`) (`KismetMathLibrary.MakeTransform` (`self.K2_GetActorLocation`) (`KismetMathLibrary.MakeRotator` _returnvalue_roll _returnvalue_pitch (`KismetMathLibrary.RandomFloatInRange` (- _returnvalue_yaw _zspawnrotationoffset) (+ _returnvalue_yaw _zspawnrotationoffset)))) "Undefined" "SelectDefaultAtRuntime" null null))
  (bind _asbp_koso_sparato (cast `/Game/Blueprints/Traps/BP_KosoSparato` _returnvalue))
  (`/Game/Blueprints/Traps/BP_KosoSparato.SetMesh` _asbp_koso_sparato (`self.ShootStaticMesh`) (`self.StaticMeshRotation`) (* (`KismetMathLibrary.MakeVector` 1.0 1.0 1.0) (`KismetMathLibrary.RandomFloatInRange` (`self.MinScaleMultiply`) (`self.MaxScaleMultipluy`))))
  (`/Game/Blueprints/Traps/BP_KosoSparato.AddImpulse` _asbp_koso_sparato (`KismetMathLibrary.RandomFloatInRange` (`self.MinForce Impulse`) (`self.MaxForce Impulse`)) false true))

(event `self.ReceiveTick`
  (params (DeltaSeconds :type "Float (single-precision)")))

(fn `DestroyNearActor`
  (bind _outactors (`KismetSystemLibrary.SphereOverlapActors` (`self.K2_GetActorLocation`) (`self.DeathArea`) (`|MakeArray` "ObjectTypeQuery7" :!type "EObjectTypeQuery Enum") "BP_KosoSparone_C" (`|MakeArray` self :!type "Actor Object Reference")))
  (for _array_element _outactors
    (`self.K2_DestroyActor` _array_element)))

(fn `UserConstructionScript`)