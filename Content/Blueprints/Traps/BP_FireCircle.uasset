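; Fire ring trap that awards score when its inner mesh is overlapped, unless the ring's collision registers a hit.
; A spawned VFX ring follows the actor, and the overlap waits briefly before scoring so a ring hit can cancel it.
; Points scale with the impact direction's alignment to the scene's forward axis, snapping to maximum when closely aligned.
; Scoring or hitting plays a timeline that shrinks effect and collision, then destroys the actor.
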(event `self.ReceiveTick`
  (params (DeltaSeconds :type "Float (single-precision)"))
  (`SceneComponent.K2_SetWorldLocationAndRotation` (`self.Effettino`) (`self.K2_GetActorLocation`) (`self.K2_GetActorRotation`) false false))

(event `self.ReceiveBeginPlay`
  (bind _asgm_base (cast `/Game/Blueprints/GameModes/GM_Base` (`GameplayStatics.GetGameMode`)))
  (set `self.As GM Base` _asgm_base)
  (bind _returnvalue (`NiagaraFunctionLibrary.SpawnSystemAtLocation` "/Game/VFX/VFX_FireRing.VFX_FireRing" (`self.K2_GetActorLocation`) (struct :`Pitch` 90.0 :`Yaw` 180.0 :`Roll` 11111.0)))
  (set `self.Effettino` _returnvalue)
  (set `self.BaseScale` (`SceneComponent.K2_GetComponentScale` (`self.RingCollision`)))
  (`SceneComponent.SetHiddenInGame` (`self.RingCollision`) true false))

(event `self.StaticMesh.OnComponentBeginOverlap`
  (params (OverlappedComponent :type "PrimitiveComponent Object Reference") (OtherActor :type "Actor Object Reference") (OtherComp :type "PrimitiveComponent Object Reference") (OtherBodyIndex :type Integer) (bFromSweep :type Boolean) (SweepResult :type "HitResult Structure (by ref)"))
  ;[1 1 1] Da fixare
  (`/Engine/EditorBlueprintResources/StandardMacros.DoOnce` false
    (:`Completed`
      (`KismetSystemLibrary.Delay` 0.2)
      (if (not (`self.NoScore`))
        (`/Game/Blueprints/Characters/Component/BPC_Score.AddScore` (`/Game/Blueprints/Characters/BP_BaseCharacter.BPC_Score` (`/Game/Blueprints/GameModes/GM_Base.CharacterReference` (`self.As GM Base`))) (`self.DistanceFromCenter` SweepResult_ImpactPoint) (`self.Multipy`))
        (`GameplayStatics.PlaySound2D` "/Game/Assets/Sounds/Wav/CharacterSounds/FunghiBoom.FunghiBoom" 0.02 1.0 0.6 null null)
        (bind (_direction _newtrack_0) (`Timeline|Timeline` :!via `PlayFromStart` :!label _label)
          (:`Update`
            (`self.RemoveCircle` _newtrack_0))
          (:`Finished`
            (`self.K2_DestroyActor`)))))))

(event `self.RingCollision.OnComponentHit`
  (params (HitComponent :type "PrimitiveComponent Object Reference") (OtherActor :type "Actor Object Reference") (OtherComp :type "PrimitiveComponent Object Reference") (NormalImpulse :type "Vector Structure") (Hit :type "HitResult Structure (by ref)"))
  ;[1 1 1] Da fixare
  (set `self.NoScore` true)
  (goto _label :!via `PlayFromStart`))

(fn `DistanceFromCenter`
  (params (point :type "Vector Structure"))
  (returns (Score :type Integer))
  (bind _returnvalue (`KismetMathLibrary.Abs` (`KismetMathLibrary.Dot_VectorVector` (`KismetMathLibrary.Normal` (- (`SceneComponent.K2_GetComponentLocation` (`self.Scene`)) point)) (`SceneComponent.GetForwardVector` (`self.Scene`)))))
  (return (`KismetMathLibrary.FFloor` (`KismetMathLibrary.SelectFloat` (`self.Score_max`) (`KismetMathLibrary.Lerp` (`self.Score`) (`self.Score_max`) _returnvalue) (> _returnvalue 0.8)))))

(fn `RemoveCircle`
  (params (Alpha :type "Float (double-precision)"))
  (`FXSystemComponent.SetFloatParameter` (`self.Effettino`) "User.Radius" (`KismetMathLibrary.Lerp` 120.0 0.0 Alpha))
  (`SceneComponent.SetWorldScale3D` (`self.RingCollision`) (`KismetMathLibrary.VLerp` (`self.BaseScale`) (0.0 0.0 0.0) Alpha)))

(fn `UserConstructionScript`)