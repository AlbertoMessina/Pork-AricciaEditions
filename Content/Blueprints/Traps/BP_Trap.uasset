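; BP_Trap is a trap whose static mesh slides sideways between two points along its right vector.
; On BeginPlay it caches both endpoints at plus and minus Delta from the mesh's starting location, then halves the timeline play rate.
; After a random delay of up to about one second, the timeline lerps the mesh between them without sweeping, so the movement does no collision checks.
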(event `self.ReceiveBeginPlay`
  (bind _staticmesh (`self.StaticMesh`))
  (bind _staticmesh_2 (`self.StaticMesh`))
  (set `self.PosiivePositoin` (+ (`SceneComponent.K2_GetComponentLocation` _staticmesh_2) (* (`SceneComponent.GetRightVector` _staticmesh_2) (`self.Delta`))))
  (set `self.NegaiivePositoin` (- (`SceneComponent.K2_GetComponentLocation` _staticmesh) (* (`SceneComponent.GetRightVector` _staticmesh) (`self.Delta`))))
  (`TimelineComponent.SetPlayRate` (`self.Timeline`) (/ 1.0 2.0))
  (`KismetSystemLibrary.Delay` (`KismetMathLibrary.FClamp` (`KismetMathLibrary.RandomFloat`) 0.0 2.2))
  (bind (_direction _newtrack_0) (`Timeline|Timeline` :`NewTime` 0.5)
    (:`Update`
      (`SceneComponent.K2_SetWorldLocation` (`self.StaticMesh`) (`KismetMathLibrary.VLerp` (`self.PosiivePositoin`) (`self.NegaiivePositoin`) _newtrack_0) false false))))

(fn `UserConstructionScript`)