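; GM_Base is a base game mode Blueprint that caches references to the player character, its HUD and the character info widget.
; On BeginPlay it casts player 0's character and HUD to BP_BaseCharacter and BP_BaseHUD, stopping if either cast fails.
; It then binds an event to the HUD's widget-created notification.
; SetCharacterInfoReference copies the HUD's CharacterInfoWidget into the game mode.
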(event `self.ReceiveBeginPlay`
  (bind _asbp_base_character (cast `/Game/Blueprints/Characters/BP_BaseCharacter` (`GameplayStatics.GetPlayerCharacter` 0)))
  (set `self.CharacterReference` _asbp_base_character)
  (bind _asbp_base_hud (cast `/Game/Blueprints/BP_BaseHUD` (`PlayerController.GetHUD` (`GameplayStatics.GetPlayerController` 0))))
  (bind _output_get (set `self.As BP Base HUD` _asbp_base_hud))
  (add `/Game/Blueprints/BP_BaseHUD.CreatedWidget` _output_get (`|CreateDelegate` :!event `SetCharacterInfoReference`)))

(fn `SetCharacterInfoReference`
  (set `self.Character Info Widget` (`/Game/Blueprints/BP_BaseHUD.Character Info Widget` (`self.As BP Base HUD`))))

(fn `UserConstructionScript`)