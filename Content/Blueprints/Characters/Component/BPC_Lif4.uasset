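; BPC_Lif4 is a character component that tracks life as a counter, starting at MaxLife on BeginPlay.
; ReduceLife takes away one point and sets the IsDeath flag from whether CurrentLife is zero or below.
; IncreseLife adds one point without capping at MaxLife or updating IsDeath, and GetCurrentLife returns the current count.
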(event `self.ReceiveBeginPlay`
  (set `self.CurrentLife` (`self.MaxLife`)))

(fn `GetCurrentLife`
  (returns (CurrentLife :type Integer))
  (return (`self.CurrentLife`)))

(fn `IncreseLife`
  (`/Engine/EditorBlueprintResources/StandardMacros.IncrementInt` (`self.CurrentLife`)))

(fn `ReduceLife`
  (bind _result (`/Engine/EditorBlueprintResources/StandardMacros.DecrementInt` (`self.CurrentLife`))
    (:`  `
      (bind _output_get (set `self.CurrentLife` _result))
      (set `self.isDeath` (<= _output_get 0)))))