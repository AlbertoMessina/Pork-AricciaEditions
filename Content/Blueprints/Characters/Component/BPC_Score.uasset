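; Score component, likely for a character, that tracks points, a capped multiplier and a perfect-hit count.
; AddScore raises the multiplier and perfect count, then adds floored, multiplied points to the score.
; UpdateMultiply accumulates up to a maximum and derives its percentage; ResetUpdateCount zeroes the count and passes zero to it, which adds nothing rather than clearing it.
; Tick prints all four values as debug text.
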(event `self.ReceiveBeginPlay`)

(event `self.ReceiveTick`
  (params (DeltaSeconds :type "Float (single-precision)"))
  (set `self.Delta Seconds` DeltaSeconds)
  (`KismetSystemLibrary.PrintString` (`KismetStringLibrary.Concat_StrStr` "Score :" (`KismetStringLibrary.Conv_IntToString` (`self.Score`))))
  (`KismetSystemLibrary.PrintString` (`KismetStringLibrary.Concat_StrStr` "Multy :" (`KismetStringLibrary.Conv_DoubleToString` (`self.Multiply`))))
  (`KismetSystemLibrary.PrintString` (`KismetStringLibrary.Concat_StrStr` "PercentCounbt :" (`KismetStringLibrary.Conv_DoubleToString` (`KismetMathLibrary.Conv_IntToDouble` (`self.PercetCount`)))))
  (`KismetSystemLibrary.PrintString` (`KismetStringLibrary.Concat_StrStr` "Multiply percentage :" (`KismetStringLibrary.Conv_DoubleToString` (`self.MultiplayPercentage`)))))

(fn `AddScore`
  (params (Score :type Integer) (Multiply :type "Float (double-precision)"))
  (`self.UpdateMultiply` Multiply)
  (`self.UpdatePerfectCount`)
  (set `self.Score` (+ (`self.Score`) (`KismetMathLibrary.FFloor` (* Score (`self.Multiply`))))))

(fn `ResetUpdateCount`
  (set `self.PercetCount` 0)
  (`self.UpdateMultiply` 0.0))

(fn `UpdateMultiply`
  (params (Multiply :type "Float (double-precision)"))
  (if (< Multiply (`self.MultiplyMax`))
    (set `self.Multiply` (+ Multiply (`self.Multiply`)))
    (set `self.MultiplayPercentage` (/ (`self.Multiply`) (`self.MultiplyMax`)))
    (else
      (set `self.Multiply` (`self.MultiplyMax`)))))

(fn `UpdatePerfectCount`
  (bind _result (`/Engine/EditorBlueprintResources/StandardMacros.IncrementInt` (`self.PercetCount`))
    (:`  `
      (set `self.PercetCount` _result))))