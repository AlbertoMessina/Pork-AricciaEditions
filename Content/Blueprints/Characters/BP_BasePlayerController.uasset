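; Base player controller that handles input setup, character possession and pause toggling through GM_Base.
; On BeginPlay it adds the base Enhanced Input mapping context, caches the game mode and binds to its character-spawn dispatcher.
; When the character spawns, it possesses the game mode's character reference and broadcasts the possession.
; Look input is relayed through its own dispatcher, and the M key toggles pause on the game mode.
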(event `Key|M` :paused true
  (params (Key :type "Key Structure"))
  (bind _as_gm_base (`self.As GM Base`))
  (:`Pressed`
    (if (`GameplayStatics.IsGamePaused`)
      (`/Game/Blueprints/GameModes/GM_Base.ResumePause` _as_gm_base)
      (else
        (`/Game/Blueprints/GameModes/GM_Base.PauseGame` _as_gm_base)))))

(event `self.ReceiveBeginPlay`
  (`|ExecutionSequence`
    (:`then_0`
      (`EnhancedInputSubsystemInterface.AddMappingContext` (subsystem `EnhancedInputLocalPlayerSubsystem`) "/Game/Blueprints/Inputs/IMC_Base.IMC_Base" 0 (struct)))
    (:`then_1`
      (bind _asgm_base (cast `/Game/Blueprints/GameModes/GM_Base` (`GameplayStatics.GetGameMode`)))
      (bind _output_get (set `self.As GM Base` _asgm_base))
      (add `/Game/Blueprints/GameModes/GM_Base.OnCharacterSpawn` _output_get (`|CreateDelegate` :!event `OnCharaceterSpawn`)))))

(event `EnhancedInput|/Game/Blueprints/Inputs/IA_Look`
  (params (ActionValue :type "Vector2D Structure") (ElapsedSeconds :type "Float (double-precision)") (TriggeredSeconds :type "Float (double-precision)") (InputAction :type "InputAction Object Reference" :default "/Game/Blueprints/Inputs/IA_Look.IA_Look"))
  (:`Triggered`
    (`self.InputLook`)))

(event `OnCharaceterSpawn`
  (`self.Possess` (`/Game/Blueprints/GameModes/GM_Base.CharacterReference` (`self.As GM Base`)))
  (`self.OnPossessCharacter`))

(fn `UserConstructionScript`)