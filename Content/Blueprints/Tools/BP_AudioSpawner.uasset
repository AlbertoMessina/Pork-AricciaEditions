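; BP_AudioSpawner plays environment music and ambience through a MetaSound component, reacting to the player character's running.
; BeginPlay passes in background songs, triggers ambient playback and binds the character's run events.
; Run start resets base pitch and enables Tick, which feeds speed percentage into the MetaSound, while ragdoll stop triggers a low-pass.
; Run stop only prints; the interpolated volume/pitch fade function has no caller here.
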(event `self.ReceiveBeginPlay`
  (`AudioParameterControllerInterface.SetObjectArrayParameter` (`self.MS_Environments`) "BackgroundSongs" (`self.BackgroundSong`))
  (`AudioParameterControllerInterface.SetTriggerParameter` (`self.MS_Environments`) "Play Ambient")
  (bind _asbp_base_character (cast `/Game/Blueprints/Characters/BP_BaseCharacter` (`GameplayStatics.GetPlayerCharacter` 0)))
  (bind _output_get (set `self.As BP Base Character` _asbp_base_character))
  (add `/Game/Blueprints/Characters/BP_BaseCharacter.StartRun` _output_get (delegate `StartSound`))
  ;[0.0213 1 0.1871] Stop Audio
  (add `/Game/Blueprints/Characters/BP_BaseCharacter.StopRun` _output_get (delegate `StopSound`))
  ;[1 1 1] FORCE STOP AUDIO
  (add `/Game/Blueprints/Characters/BP_BaseCharacter.StopRunRagdoll` _output_get (delegate `RagdollStop`)))

(event `StopSound`
  ;[0.0213 1 0.1871] Stop Audio
  (`KismetSystemLibrary.PrintString` "Stop Audio"))

(event `StartSound`
  ;[1 0.592 0.0355] Start Sound
  (`AudioParameterControllerInterface.SetTriggerParameter` (`self.MS_Environments`) "SetBasePitch")
  (add `AudioComponent.OnAudioPlaybackPercent` (`self.MS_Environments`) (`|CreateDelegate` :!event `SetSourceTime `))
  (`self.SetActorTickEnabled` true))

(event `self.ReceiveTick`
  (params (DeltaSeconds :type "Float (single-precision)"))
  (`AudioParameterControllerInterface.SetFloatParameter` (`self.MS_Environments`) "PlayerSpeedPercentage" (`/Game/Blueprints/Characters/BP_BaseCharacter.SpeedPercentage` (`self.As BP Base Character`))))

(event `RagdollStop`
  ;[1 1 1] FORCE STOP AUDIO
  (`AudioParameterControllerInterface.SetTriggerParameter` (`self.MS_Environments`) "StartLowPass"))

(fn `SetInterpolationParameter`
  (params (Target :type "Float (double-precision)") (`Interp Speed` :type "Float (double-precision)") (PitchIntensity :type "Float (double-precision)"))
  (set `self.MaxVoluime` Target)
  (set `self.Interp Speed` `Interp Speed`)
  (set `self.PitchIntensity` PitchIntensity))

(fn `SetSourceTime `
  (params (PlayingSoundWave :type "SoundWave Object Reference") (PlaybackPercent :type "Float (single-precision)"))
  (set `self.SoundTime` (* (`SoundBase.Duration` PlayingSoundWave) PlaybackPercent)))

(fn `Spawn Audio`
  (params (InputPin :type "Float (single-precision)"))
  (bind _startvolume (`self.StartVolume`))
  (bind _returnvalue (`KismetMathLibrary.FInterpTo` (`self.StartVolume`) (`self.MaxVoluime`) InputPin (`self.Interp Speed`)))
  (`AudioComponent.SetVolumeMultiplier` (`self.MS_Environments`) _startvolume)
  ;[1 1 1] Interessante
  (`AudioComponent.SetPitchMultiplier` (`self.MS_Environments`) (`KismetMathLibrary.FClamp` (* _startvolume (`self.PitchIntensity`))))
  (set `self.StartVolume` _returnvalue)
  (if (== _returnvalue (`self.MaxVoluime`))
    (`self.SetActorTickEnabled` false)))

(fn `UserConstructionScript`)