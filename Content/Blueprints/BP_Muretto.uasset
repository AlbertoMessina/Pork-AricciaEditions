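; BP_Muretto is a destructible low wall built on a Geometry Collection, topped with a flame and reacting to its first impact.
; BeginPlay spawns a collisionless fire mesh and positions it above the collection from component bounds.
; The Box's first hit triggers OnGetHit on a BP_BaseCharacter, then after a short delay switches wall collision to Overlap.
; Any other first hitter makes the Box and collection ignore all channels immediately.
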(event `self.ReceiveBeginPlay`
  (bind (_origin _boxextent) (`KismetSystemLibrary.GetComponentBounds` (`self.GeometryCollectionComponent`)))
  (bind _result (`/Engine/EditorBlueprintResources/StandardMacros.NegateFloat` (.z _boxextent))
    (:`  `
      (bind _returnvalue (`AddComponent|NODE_AddStaticMeshComponent-0` :`RelativeTransform` (`KismetMathLibrary.MakeTransform` (`self.K2_GetActorLocation`) (struct :`Yaw` 90.0 :`Roll` 90.0) (0.5 0.5 0.5))))
      (`PrimitiveComponent.SetCollisionEnabled` _returnvalue "NoCollision")
      (`StaticMeshComponent.SetStaticMesh` _returnvalue (`self.Flame`))
      (`PrimitiveComponent.SetMaterial` _returnvalue 0 "/Game/Materials/MI_Fire.MI_Fire")
      (`SceneComponent.K2_SetWorldLocation` _returnvalue (+ (+ _origin (`KismetMathLibrary.MakeVector` 0.0 (/ (.y _boxextent) 2.0) _result)) (`KismetMathLibrary.MakeVector` 0.0 0.0 (.z (`.BoxExtent` (`KismetSystemLibrary.GetComponentBounds` _returnvalue))))) false false))))

(event `self.Box.OnComponentHit`
  (params (HitComponent :type "PrimitiveComponent Object Reference") (OtherActor :type "Actor Object Reference") (OtherComp :type "PrimitiveComponent Object Reference") (NormalImpulse :type "Vector Structure") (Hit :type "HitResult Structure (by ref)"))
  (`/Engine/EditorBlueprintResources/StandardMacros.DoOnce` false
    (:`Completed`
      (bind _asbp_base_character (cast `/Game/Blueprints/Characters/BP_BaseCharacter` OtherActor)
        (:`then`
          (`/Game/Blueprints/Characters/BP_BaseCharacter.OnGetHit` _asbp_base_character OtherActor Hit_Normal 0.2)
          (`KismetSystemLibrary.Delay` 0.5)
          (`self.SetBlockPlayer`))
        (:`CastFailed`
          (`PrimitiveComponent.SetCollisionResponseToAllChannels` (`self.Box`) "ECR_Ignore")
          (`PrimitiveComponent.SetCollisionResponseToAllChannels` (`self.GeometryCollectionComponent`) "ECR_Ignore"))))))

(fn `SetBlockPlayer`
  (`PrimitiveComponent.SetCollisionResponseToAllChannels` (`self.Box`) "ECR_Overlap")
  (`PrimitiveComponent.SetCollisionResponseToAllChannels` (`self.GeometryCollectionComponent`) "ECR_Overlap"))

(fn `UserConstructionScript`)