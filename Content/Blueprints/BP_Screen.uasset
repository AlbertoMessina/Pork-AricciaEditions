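; BP_Screen is a hidden actor that plays a video with sound when the player character has one life left.
; On BeginPlay it links MediaSound to the MediaPlayer, opens a green-screen video source and, after a short delay, binds to the one-life-left event on GM_Base's character reference.
; When that fires and nothing is playing, it reveals itself, plays the clip with a logarithmic audio fade-in, then hides again after the clip's duration.
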(event `self.ReceiveBeginPlay`
  (`self.SetActorHiddenInGame` (`self.Hidden`))
  (`MediaSoundComponent.SetMediaPlayer` (`self.MediaSound`) (`self.MediaPlayer`))
  (`MediaPlayer.OpenSource` (`self.MediaPlayer`) "/Game/Movies/Big_enough_green_screen.Big_enough_green_screen")
  (`KismetSystemLibrary.Delay` 0.2)
  (bind _asgm_base (cast `/Game/Blueprints/GameModes/GM_Base` (`GameplayStatics.GetGameMode`)))
  (add `/Game/Blueprints/Characters/BP_BaseCharacter.OneLifeLeft` (`/Game/Blueprints/GameModes/GM_Base.CharacterReference` _asgm_base) (delegate `OpenSource`)))

(event `OpenSource`
  (bind _mediaplayer (`self.MediaPlayer`))
  (bind (_returnvalue_days _returnvalue_hours _returnvalue_minutes _returnvalue_seconds) (`KismetMathLibrary.BreakTimespan` (`MediaPlayer.GetDuration` _mediaplayer)))
  (if (not (`MediaPlayer.IsPlaying` _mediaplayer))
    (`self.SetActorHiddenInGame` false)
    (`MediaPlayer.Play` _mediaplayer)
    (`SynthComponent.FadeIn` (`self.MediaSound`) 6.0 1.0 0.0 "Logarithmic")
    (`KismetSystemLibrary.Delay` (`KismetMathLibrary.Conv_IntToDouble` _returnvalue_seconds))
    (`self.SetActorHiddenInGame` true)))

(fn `UserConstructionScript`)