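; BP_Fire is an actor that bobs vertically around its placed height, likely as a fire prop or effect.
; On BeginPlay it stores its starting Z, waits a random delay, then plays a timeline at a randomized rate so instances move out of sync.
; Each timeline update lerps Z between DeltaZ above and below that height, keeping X and Y unchanged.
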(event `self.ReceiveBeginPlay`
  (bind (_returnvalue_x _returnvalue_y) (`KismetMathLibrary.BreakVector` (`self.K2_GetActorLocation`)))
  (bind (_returnvalue_x_2 _returnvalue_y_2 _returnvalue_z) (`KismetMathLibrary.BreakVector` (`self.K2_GetActorLocation`)))
  (set `self.BeginZ` _returnvalue_z)
  (`KismetSystemLibrary.Delay` (`KismetMathLibrary.RandomFloatInRange` 0.0 2.0))
  (`TimelineComponent.SetPlayRate` (`self.Timeline`) (/ 1.0 (`KismetMathLibrary.RandomFloatInRange` 0.5 2.0)))
  (bind (_direction _newtrack_0) (`Timeline|Timeline`)
    (:`Update`
      (`self.K2_SetActorLocation` (`KismetMathLibrary.MakeVector` _returnvalue_x _returnvalue_y (`KismetMathLibrary.Lerp` (+ (`self.DeltaZ`) (`self.BeginZ`)) (- (`self.BeginZ`) (`self.DeltaZ`)) _newtrack_0))))))

(fn `UserConstructionScript`)